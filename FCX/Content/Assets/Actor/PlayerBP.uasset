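; Player actor Blueprint that turns one player's input into cursor movement through a shared PlayerManager reference.
; MoveForward and MoveRight axes each build a single-axis vector scaled by the manager's Power, with the forward axis inverted, and pass it with PlayerID to CursorMove.
; The Red action only prints PlayerID and the manager's Test value for debugging.
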(event EventBeginPlay)

(event Collision|EventActorBeginOverlap
  (params (OtherActor :type Actor%20Object%20Reference)))

(event EventTick
  (params (DeltaSeconds :type Float%20%28single-precision%29)))

(event Input|ActionEvents|InputActionRed
  (params (Key :type Key%20Structure :default "None"))
  (:Pressed
    (Development|PrintString (Utilities|String|ToString(Integer) (Variables|Default|GetPlayerID)) true true "(R=1.000000,G=0.000000,B=0.053313,A=1.000000)")
    (Development|PrintString (Variables|/Game/Assets/Manager/PlayerManager.PlayerManager_C|GetTest (Variables|Default|GetPlayerManagerRef)) true true "(R=1.000000,G=0.023239,B=0.000000,A=1.000000)")))

(event Input|AxisEvents|InputAxisMoveForward
  (params (AxisValue :type Float%20%28single-precision%29))
  (bind _output_get (Variables|Default|SetMovement (Math|Vector2D|MakeVector2D 0.0 (* AxisValue (* (Variables|/Game/Assets/Manager/PlayerManager.PlayerManager_C|GetPower (Variables|Default|GetPlayerManagerRef)) -1.0)))))
  (Default|CursorMove (Variables|Default|GetPlayerManagerRef) (Variables|Default|GetPlayerID) _output_get))

(event Input|AxisEvents|InputAxisMoveRight
  (params (AxisValue :type Float%20%28single-precision%29))
  (bind _output_get (Variables|Default|SetMovement (Math|Vector2D|MakeVector2D (* (Variables|/Game/Assets/Manager/PlayerManager.PlayerManager_C|GetPower (Variables|Default|GetPlayerManagerRef)) AxisValue) 0.0)))
  (Default|CursorMove (Variables|Default|GetPlayerManagerRef) (Variables|Default|GetPlayerID) _output_get))

(fn ConstructionScript)